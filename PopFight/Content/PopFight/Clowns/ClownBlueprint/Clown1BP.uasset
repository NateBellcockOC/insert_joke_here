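; Clown1BP is a clown sprite Blueprint for PopFight that shows a laugh reaction on demand.
; The MakeMeLaugh event sets Clown1Sprite to one of three laugh sprites picked at random, waits four seconds, then calls the Nothing event.
; Nothing restores the straight-faced sprite, and the construction script is empty.
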(event EventMakeMeLaugh
  (Rendering|Components|Sprite|SetSprite (Variables|Default|GetClown1Sprite) (.OutItem (Utilities|Array|Random (Utilities|Array|MakeArray (Variables|Default|GetLaugh1) (Variables|Default|GetLaugh2) (Variables|Default|GetLaugh3)))))
  (Utilities|FlowControl|Delay 4.0)
  (CallFunction|Nothing))

(event EventNothing
  (Rendering|Components|Sprite|SetSprite (Variables|Default|GetClown1Sprite) "/Game/PopFight/Clowns/Sprites/Clown1_straight_Sprite.Clown1_straight_Sprite"))

(fn ConstructionScript)