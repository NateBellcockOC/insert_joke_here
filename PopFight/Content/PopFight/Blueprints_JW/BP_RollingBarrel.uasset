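; BP_RollingBarrel is a short-lived barrel hazard that reacts to contact with players.
; On spawn it pushes its capsule with an impulse along world forward, then after a short delay spawns confetti at the barrel, activates Bomp15 and destroys itself.
; Overlapping an actor tagged Player calls PopMessage on that actor and destroys the barrel immediately, skipping the timed confetti burst.
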(event OnComponentBeginOverlap(Capsule)
  (params (OverlappedComponent :type Primitive%20Component%20Object%20Reference) (OtherActor :type Actor%20Object%20Reference) (OtherComp :type Primitive%20Component%20Object%20Reference) (OtherBodyIndex :type Integer) (bFromSweep :type Boolean) (SweepResult :type Hit%20Result%20Structure%20%28by%20ref%29))
  (if (Actor|ActorHasTag OtherActor "Player")
    (Class|PlayerMechanics|Pop(Message) OtherActor)
    (Actor|DestroyActor)))

(event EventBeginPlay
  (Physics|AddImpulse (Variables|Default|GetCapsule) (* (Math|Vector|GetForwardVector "0, 0, 0") 1e+02) "None" false)
  (Utilities|FlowControl|Delay 1.5)
  (Niagara|SpawnSystematLocation "/Game/PopFight/Particles/Confetti/P_Confetti.P_Confetti" (Transformation|GetWorldLocation (Variables|Default|GetBarrel)))
  (Components|Activation|Activate (Variables|Default|GetBomp_15) false)
  (Actor|DestroyActor))

(event Collision|EventActorBeginOverlap
  (params (OtherActor :type Actor%20Object%20Reference)))

(event EventTick
  (params (DeltaSeconds :type Float%20%28single-precision%29)))

(fn ConstructionScript)