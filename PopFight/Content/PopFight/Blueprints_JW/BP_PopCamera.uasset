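; BP_PopCamera is a shared camera rig that follows the first two player characters and zooms with their separation.
; Each tick it moves a Cube toward their average location using a lerp with alpha 1.5, which extrapolates past the midpoint.
; A nested loop gathers the distance to player 1, and the maximum, clamped between MinArmLength and MaxArmLength, sets the SpringArm length.
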(event EventTick
  (params (DeltaSeconds :type Float%20%28single-precision%29))
  (bind _returnvalue (Game|GetPlayerCharacter 0))
  (bind _returnvalue_2 (Game|GetPlayerCharacter 1))
  (bind _array (Utilities|Array|MakeArray _returnvalue _returnvalue_2))
  ;[1 1 1] Update Camera Position
  (Variables|Default|SetPreviousLocation (Transformation|GetWorldLocation (Variables|Default|GetCube)))
  (bind _returnvalue_3 (Class|GameplayStatics|GetActorArrayAverageLocation (Utilities|Array|MakeArray (Game|GetPlayerCharacter 0) (Game|GetPlayerCharacter 1))))
  (Transformation|SetWorldLocation (Variables|Default|GetCube) (Math|Vector|Lerp(Vector) (Variables|Default|GetPreviousLocation) _returnvalue_3 1.5) false false)
  ;[1 1 1] Calculate Camera Distance
  (for (_array_element _array_index) _array
    (Variables|Default|SetPlayer _array_element)
    (for _index (range (+ _array_index 1) (- (Utilities|Array|Length _array) 1))
      (Utilities|Array|Add (Variables|Default|GetDistance) (Transformation|GetDistanceTo (Variables|Default|GetPlayer) (Game|GetPlayerCharacter 1)))))
  ;[1 1 1] Update camera distance
  (Variables|/Script/Engine.SpringArmComponent|SetTargetArmLength (Variables|Default|GetSpringArm) (Math|Float|Clamp(Float) (.MaxValue (Math|Float|MaxOfFloatArray (Variables|Default|GetDistance))) (Variables|Default|GetMinArmLength) (Variables|Default|GetMaxArmLength)))
  (Utilities|Array|Clear (Variables|Default|GetDistance)))

(fn ConstructionScript)