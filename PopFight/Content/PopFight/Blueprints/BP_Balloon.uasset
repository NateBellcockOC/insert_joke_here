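; BP_Balloon is a balloon actor in PopFight that pops when any actor overlaps it, awarding points.
; On overlap it sends a respawn message to one of two spawn references, chosen by IsRespawnable, then plays a pop sound and confetti at its sphere.
; It passes PointsWorth to the overlapping actor through GetPointsMessage, then destroys itself.
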(event EventBeginPlay)

(event Collision|EventActorBeginOverlap
  (params (OtherActor :type Actor%20Object%20Reference))
  (bind _sphere (Variables|Default|GetSphere))
  (bind _returnvalue (Transformation|GetWorldLocation _sphere))
  (Utilities|FlowControl|Sequence
    (:then_0
      (if (Variables|Default|GetIsRespawnable)
        (Class|BPIBalloonRespawn|Respawn(Message) (Variables|Default|Getspawn))
        (else
          (Class|BPIBalloonRespawn|Respawn(Message) (Variables|Default|GetspawnNew))))
      (Audio|PlaySoundatLocation "/Game/PopFight/Audio/Lil_Pop_1.Lil_Pop_1" _returnvalue "0, 0, 0" 1.0 1.0 0.0 0 0 0 0)
      (Niagara|SpawnSystematLocation "/Game/PopFight/Particles/Confetti/P_Confetti.P_Confetti" _returnvalue)
      (Class|BPIPoints|GetPoints(Message) OtherActor (Variables|Default|GetpointsWorth)))
    (:then_1
      (Actor|DestroyActor))))

(event EventTick
  (params (DeltaSeconds :type Float%20%28single-precision%29)))

(fn ConstructionScript)