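; Spawner actor that fills a square area with balloons at a set height for PopFight.
; On BeginPlay it spawns ten balloons at random X/Y within shared Min/Max world bounds, with random rotation (roll reuses those bounds).
; Its Respawn event spawns one BP_Balloon_Spawn_Temp the same way, but with full-circle random roll.
; Each spawned actor receives this spawner in its SpawnNew reference.
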(event EventBeginPlay
  (bind _min (Variables|Default|Getmin))
  (bind _max (Variables|Default|Getmax))
  (bind _returnvalue (Math|Random|RandomFloatinRange _min _max))
  (for _index (range 0 9)
    (bind _returnvalue_2 (Game|SpawnActorfromClass "/Game/PopFight/Blueprints/BP_Balloon.BP_Balloon_C" (Math|Transform|MakeTransform (Math|Vector|MakeVector _returnvalue (Math|Random|RandomFloatinRange (Variables|Default|Getmin) (Variables|Default|Getmax)) (Variables|Default|Getheight)) (Math|Rotator|MakeRotator _returnvalue (Math|Random|RandomFloatinRange 0.0 3.6e+02) (Math|Random|RandomFloatinRange 0.0 3.6e+02)) "1.000000,1.000000,1.000000") "Undefined" "MultiplyWithRoot" 0 0))
    (Variables|/Game/PopFight/Blueprints/BP_Balloon.BP_Balloon_C|SetspawnNew _returnvalue_2 self)))

(event Collision|EventActorBeginOverlap
  (params (OtherActor :type Actor%20Object%20Reference)))

(event EventTick
  (params (DeltaSeconds :type Float%20%28single-precision%29)))

(event EventRespawn
  (bind _returnvalue (Game|SpawnActorfromClass "/Game/PopFight/Blueprints/BP_Balloon_Spawn_Temp.BP_Balloon_Spawn_Temp_C" (Math|Transform|MakeTransform (Math|Vector|MakeVector (Math|Random|RandomFloatinRange (Variables|Default|Getmin) (Variables|Default|Getmax)) (Math|Random|RandomFloatinRange (Variables|Default|Getmin) (Variables|Default|Getmax)) (Variables|Default|Getheight)) (Math|Rotator|MakeRotator (Math|Random|RandomFloatinRange 0.0 3.6e+02) (Math|Random|RandomFloatinRange 0.0 3.6e+02) (Math|Random|RandomFloatinRange 0.0 3.6e+02)) "1.000000,1.000000,1.000000") "Undefined" "MultiplyWithRoot" 0 0))
  (Variables|/Game/PopFight/Blueprints/BP_Balloon_Spawn_Temp.BP_Balloon_Spawn_Temp_C|SetspawnNew _returnvalue self))

(fn ConstructionScript)