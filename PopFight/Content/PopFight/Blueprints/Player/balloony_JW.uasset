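; Player balloon animal in PopFight, hopped and turned by combining four Enhanced Input leg actions.
; All leg presses share one DoOnce, wait briefly to catch chords, then map the held combination to Move if grounded.
; Move applies capsule impulses and sets control yaw, while a downward trace on Tick sets CanJump.
; K messages ClownInterface actors to laugh; the looping GroundCheck timer event is empty, and debug print and trace drawing remain on.
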(event Custom|Ground%20Check)

(event Input|EnhancedActionEvents|EnhancedInputActionFornt_Left_Leg
  (params (ActionValue :type Boolean) (ElapsedSeconds :type Float%20%28double-precision%29) (TriggeredSeconds :type Float%20%28double-precision%29) (InputAction :type Input%20Action%20Object%20Reference :default "/Game/PopFight/Blueprints/Player/input/Fornt_Left_Leg.Fornt_Left_Leg"))
  (bind _returnvalue (Input|EnhancedActionValues|GetBack_Left_Leg))
  (bind _returnvalue_2 (Input|EnhancedActionValues|GetFornt_Left_Leg))
  (bind _returnvalue_3 (Input|EnhancedActionValues|GetFornt_Right_Leg))
  (bind _returnvalue_4 (Input|EnhancedActionValues|GetBack_Right_Leg))
  (:Started
    (Utilities|FlowControl|DoOnce false :!label _label
      (:Completed
        (Utilities|FlowControl|Delay 0.05)
        (Development|PrintString (Utilities|String|Append "FLL:" (Utilities|String|ToString(Boolean) (Input|EnhancedActionValues|GetFornt_Left_Leg)) "BLL: " (Utilities|String|ToString(Boolean) (Input|EnhancedActionValues|GetBack_Left_Leg)) "FRL: " (Utilities|String|ToString(Boolean) (Input|EnhancedActionValues|GetFornt_Right_Leg)) "BRL: " (Utilities|String|ToString(Boolean) (Input|EnhancedActionValues|GetBack_Right_Leg))))
        (if (Variables|Default|GetCan%20jump)
          (if (Math|Boolean|ANDBoolean _returnvalue_2 _returnvalue _returnvalue_3 _returnvalue_4)
            (CallFunction|Move 0.0 0.0 4.0 0.0)
            (goto _label Reset)
            (elif (Math|Boolean|ANDBoolean _returnvalue_2 _returnvalue _returnvalue_3)
              (CallFunction|Move -1.0 -1.0 3.0 0.0)
              (goto _label Reset)
              (elif (Math|Boolean|ANDBoolean _returnvalue_2 _returnvalue _returnvalue_4)
                (CallFunction|Move -1.0 1.0 3.0 0.0)
                (goto _label Reset)
                (elif (Math|Boolean|ANDBoolean _returnvalue_2 _returnvalue_3 _returnvalue_4)
                  (CallFunction|Move 1.0 -1.0 3.0 0.0)
                  (goto _label Reset)
                  (elif (Math|Boolean|ANDBoolean _returnvalue _returnvalue_3 _returnvalue_4)
                    (CallFunction|Move 1.0 1.0 3.0 0.0)
                    (goto _label Reset)
                    (elif (and _returnvalue_2 _returnvalue)
                      (CallFunction|Move -2.0 0.0 2.0 0.0)
                      (goto _label Reset)
                      (elif (and _returnvalue_2 _returnvalue_3)
                        (CallFunction|Move 0.0 -2.0 2.0 0.0)
                        (goto _label Reset)
                        (elif (and _returnvalue_2 _returnvalue_4)
                          (CallFunction|Move 0.0 0.0 0.0 1.0)
                          (goto _label Reset)
                          (elif (and _returnvalue _returnvalue_3)
                            (CallFunction|Move 0.0 0.0 0.0 -1.0)
                            (goto _label Reset)
                            (elif (and _returnvalue _returnvalue_4)
                              (CallFunction|Move 0.0 2.0 2.0 0.0)
                              (goto _label Reset)
                              (elif (and _returnvalue_3 _returnvalue_4)
                                (CallFunction|Move 2.0 0.0 2.0 0.0)
                                (goto _label Reset)
                                (elif _returnvalue_2
                                  (CallFunction|Move -1.0 -1.0 1.0 0.0)
                                  (goto _label Reset)
                                  (elif _returnvalue
                                    (CallFunction|Move -1.0 1.0 1.0 0.0)
                                    (goto _label Reset)
                                    (elif _returnvalue_3
                                      (CallFunction|Move 1.0 -1.0 1.0 0.0)
                                      (goto _label Reset)
                                      (elif _returnvalue_4
                                        (CallFunction|Move 1.0 1.0 1.0 0.0)
                                        (goto _label Reset)
                                        (else
                                          (goto _label Reset))))))))))))))))))))))

(event Input|EnhancedActionEvents|EnhancedInputActionBack_Left_Leg
  (params (ActionValue :type Boolean) (ElapsedSeconds :type Float%20%28double-precision%29) (TriggeredSeconds :type Float%20%28double-precision%29) (InputAction :type Input%20Action%20Object%20Reference :default "/Game/PopFight/Blueprints/Player/input/Back_Left_Leg.Back_Left_Leg"))
  (bind _returnvalue (Input|EnhancedActionValues|GetBack_Left_Leg))
  (bind _returnvalue_2 (Input|EnhancedActionValues|GetFornt_Left_Leg))
  (bind _returnvalue_3 (Input|EnhancedActionValues|GetFornt_Right_Leg))
  (bind _returnvalue_4 (Input|EnhancedActionValues|GetBack_Right_Leg))
  (:Started
    (Utilities|FlowControl|DoOnce false :!label _label
      (:Completed
        (Utilities|FlowControl|Delay 0.05)
        (Development|PrintString (Utilities|String|Append "FLL:" (Utilities|String|ToString(Boolean) (Input|EnhancedActionValues|GetFornt_Left_Leg)) "BLL: " (Utilities|String|ToString(Boolean) (Input|EnhancedActionValues|GetBack_Left_Leg)) "FRL: " (Utilities|String|ToString(Boolean) (Input|EnhancedActionValues|GetFornt_Right_Leg)) "BRL: " (Utilities|String|ToString(Boolean) (Input|EnhancedActionValues|GetBack_Right_Leg))))
        (if (Variables|Default|GetCan%20jump)
          (if (Math|Boolean|ANDBoolean _returnvalue_2 _returnvalue _returnvalue_3 _returnvalue_4)
            (CallFunction|Move 0.0 0.0 4.0 0.0)
            (goto _label Reset)
            (elif (Math|Boolean|ANDBoolean _returnvalue_2 _returnvalue _returnvalue_3)
              (CallFunction|Move -1.0 -1.0 3.0 0.0)
              (goto _label Reset)
              (elif (Math|Boolean|ANDBoolean _returnvalue_2 _returnvalue _returnvalue_4)
                (CallFunction|Move -1.0 1.0 3.0 0.0)
                (goto _label Reset)
                (elif (Math|Boolean|ANDBoolean _returnvalue_2 _returnvalue_3 _returnvalue_4)
                  (CallFunction|Move 1.0 -1.0 3.0 0.0)
                  (goto _label Reset)
                  (elif (Math|Boolean|ANDBoolean _returnvalue _returnvalue_3 _returnvalue_4)
                    (CallFunction|Move 1.0 1.0 3.0 0.0)
                    (goto _label Reset)
                    (elif (and _returnvalue_2 _returnvalue)
                      (CallFunction|Move -2.0 0.0 2.0 0.0)
                      (goto _label Reset)
                      (elif (and _returnvalue_2 _returnvalue_3)
                        (CallFunction|Move 0.0 -2.0 2.0 0.0)
                        (goto _label Reset)
                        (elif (and _returnvalue_2 _returnvalue_4)
                          (CallFunction|Move 0.0 0.0 0.0 1.0)
                          (goto _label Reset)
                          (elif (and _returnvalue _returnvalue_3)
                            (CallFunction|Move 0.0 0.0 0.0 -1.0)
                            (goto _label Reset)
                            (elif (and _returnvalue _returnvalue_4)
                              (CallFunction|Move 0.0 2.0 2.0 0.0)
                              (goto _label Reset)
                              (elif (and _returnvalue_3 _returnvalue_4)
                                (CallFunction|Move 2.0 0.0 2.0 0.0)
                                (goto _label Reset)
                                (elif _returnvalue_2
                                  (CallFunction|Move -1.0 -1.0 1.0 0.0)
                                  (goto _label Reset)
                                  (elif _returnvalue
                                    (CallFunction|Move -1.0 1.0 1.0 0.0)
                                    (goto _label Reset)
                                    (elif _returnvalue_3
                                      (CallFunction|Move 1.0 -1.0 1.0 0.0)
                                      (goto _label Reset)
                                      (elif _returnvalue_4
                                        (CallFunction|Move 1.0 1.0 1.0 0.0)
                                        (goto _label Reset)
                                        (else
                                          (goto _label Reset))))))))))))))))))))))

(event Input|EnhancedActionEvents|EnhancedInputActionFornt_Right_Leg
  (params (ActionValue :type Boolean) (ElapsedSeconds :type Float%20%28double-precision%29) (TriggeredSeconds :type Float%20%28double-precision%29) (InputAction :type Input%20Action%20Object%20Reference :default "/Game/PopFight/Blueprints/Player/input/Fornt_Right_Leg.Fornt_Right_Leg"))
  (bind _returnvalue (Input|EnhancedActionValues|GetBack_Left_Leg))
  (bind _returnvalue_2 (Input|EnhancedActionValues|GetFornt_Left_Leg))
  (bind _returnvalue_3 (Input|EnhancedActionValues|GetFornt_Right_Leg))
  (bind _returnvalue_4 (Input|EnhancedActionValues|GetBack_Right_Leg))
  (:Started
    (Utilities|FlowControl|DoOnce false :!label _label
      (:Completed
        (Utilities|FlowControl|Delay 0.05)
        (Development|PrintString (Utilities|String|Append "FLL:" (Utilities|String|ToString(Boolean) (Input|EnhancedActionValues|GetFornt_Left_Leg)) "BLL: " (Utilities|String|ToString(Boolean) (Input|EnhancedActionValues|GetBack_Left_Leg)) "FRL: " (Utilities|String|ToString(Boolean) (Input|EnhancedActionValues|GetFornt_Right_Leg)) "BRL: " (Utilities|String|ToString(Boolean) (Input|EnhancedActionValues|GetBack_Right_Leg))))
        (if (Variables|Default|GetCan%20jump)
          (if (Math|Boolean|ANDBoolean _returnvalue_2 _returnvalue _returnvalue_3 _returnvalue_4)
            (CallFunction|Move 0.0 0.0 4.0 0.0)
            (goto _label Reset)
            (elif (Math|Boolean|ANDBoolean _returnvalue_2 _returnvalue _returnvalue_3)
              (CallFunction|Move -1.0 -1.0 3.0 0.0)
              (goto _label Reset)
              (elif (Math|Boolean|ANDBoolean _returnvalue_2 _returnvalue _returnvalue_4)
                (CallFunction|Move -1.0 1.0 3.0 0.0)
                (goto _label Reset)
                (elif (Math|Boolean|ANDBoolean _returnvalue_2 _returnvalue_3 _returnvalue_4)
                  (CallFunction|Move 1.0 -1.0 3.0 0.0)
                  (goto _label Reset)
                  (elif (Math|Boolean|ANDBoolean _returnvalue _returnvalue_3 _returnvalue_4)
                    (CallFunction|Move 1.0 1.0 3.0 0.0)
                    (goto _label Reset)
                    (elif (and _returnvalue_2 _returnvalue)
                      (CallFunction|Move -2.0 0.0 2.0 0.0)
                      (goto _label Reset)
                      (elif (and _returnvalue_2 _returnvalue_3)
                        (CallFunction|Move 0.0 -2.0 2.0 0.0)
                        (goto _label Reset)
                        (elif (and _returnvalue_2 _returnvalue_4)
                          (CallFunction|Move 0.0 0.0 0.0 1.0)
                          (goto _label Reset)
                          (elif (and _returnvalue _returnvalue_3)
                            (CallFunction|Move 0.0 0.0 0.0 -1.0)
                            (goto _label Reset)
                            (elif (and _returnvalue _returnvalue_4)
                              (CallFunction|Move 0.0 2.0 2.0 0.0)
                              (goto _label Reset)
                              (elif (and _returnvalue_3 _returnvalue_4)
                                (CallFunction|Move 2.0 0.0 2.0 0.0)
                                (goto _label Reset)
                                (elif _returnvalue_2
                                  (CallFunction|Move -1.0 -1.0 1.0 0.0)
                                  (goto _label Reset)
                                  (elif _returnvalue
                                    (CallFunction|Move -1.0 1.0 1.0 0.0)
                                    (goto _label Reset)
                                    (elif _returnvalue_3
                                      (CallFunction|Move 1.0 -1.0 1.0 0.0)
                                      (goto _label Reset)
                                      (elif _returnvalue_4
                                        (CallFunction|Move 1.0 1.0 1.0 0.0)
                                        (goto _label Reset)
                                        (else
                                          (goto _label Reset))))))))))))))))))))))

(event Input|EnhancedActionEvents|EnhancedInputActionBack_Right_Leg
  (params (ActionValue :type Boolean) (ElapsedSeconds :type Float%20%28double-precision%29) (TriggeredSeconds :type Float%20%28double-precision%29) (InputAction :type Input%20Action%20Object%20Reference :default "/Game/PopFight/Blueprints/Player/input/Back_Right_Leg.Back_Right_Leg"))
  (bind _returnvalue (Input|EnhancedActionValues|GetBack_Left_Leg))
  (bind _returnvalue_2 (Input|EnhancedActionValues|GetFornt_Left_Leg))
  (bind _returnvalue_3 (Input|EnhancedActionValues|GetFornt_Right_Leg))
  (bind _returnvalue_4 (Input|EnhancedActionValues|GetBack_Right_Leg))
  (:Started
    (Utilities|FlowControl|DoOnce false :!label _label
      (:Completed
        (Utilities|FlowControl|Delay 0.05)
        (Development|PrintString (Utilities|String|Append "FLL:" (Utilities|String|ToString(Boolean) (Input|EnhancedActionValues|GetFornt_Left_Leg)) "BLL: " (Utilities|String|ToString(Boolean) (Input|EnhancedActionValues|GetBack_Left_Leg)) "FRL: " (Utilities|String|ToString(Boolean) (Input|EnhancedActionValues|GetFornt_Right_Leg)) "BRL: " (Utilities|String|ToString(Boolean) (Input|EnhancedActionValues|GetBack_Right_Leg))))
        (if (Variables|Default|GetCan%20jump)
          (if (Math|Boolean|ANDBoolean _returnvalue_2 _returnvalue _returnvalue_3 _returnvalue_4)
            (CallFunction|Move 0.0 0.0 4.0 0.0)
            (goto _label Reset)
            (elif (Math|Boolean|ANDBoolean _returnvalue_2 _returnvalue _returnvalue_3)
              (CallFunction|Move -1.0 -1.0 3.0 0.0)
              (goto _label Reset)
              (elif (Math|Boolean|ANDBoolean _returnvalue_2 _returnvalue _returnvalue_4)
                (CallFunction|Move -1.0 1.0 3.0 0.0)
                (goto _label Reset)
                (elif (Math|Boolean|ANDBoolean _returnvalue_2 _returnvalue_3 _returnvalue_4)
                  (CallFunction|Move 1.0 -1.0 3.0 0.0)
                  (goto _label Reset)
                  (elif (Math|Boolean|ANDBoolean _returnvalue _returnvalue_3 _returnvalue_4)
                    (CallFunction|Move 1.0 1.0 3.0 0.0)
                    (goto _label Reset)
                    (elif (and _returnvalue_2 _returnvalue)
                      (CallFunction|Move -2.0 0.0 2.0 0.0)
                      (goto _label Reset)
                      (elif (and _returnvalue_2 _returnvalue_3)
                        (CallFunction|Move 0.0 -2.0 2.0 0.0)
                        (goto _label Reset)
                        (elif (and _returnvalue_2 _returnvalue_4)
                          (CallFunction|Move 0.0 0.0 0.0 1.0)
                          (goto _label Reset)
                          (elif (and _returnvalue _returnvalue_3)
                            (CallFunction|Move 0.0 0.0 0.0 -1.0)
                            (goto _label Reset)
                            (elif (and _returnvalue _returnvalue_4)
                              (CallFunction|Move 0.0 2.0 2.0 0.0)
                              (goto _label Reset)
                              (elif (and _returnvalue_3 _returnvalue_4)
                                (CallFunction|Move 2.0 0.0 2.0 0.0)
                                (goto _label Reset)
                                (elif _returnvalue_2
                                  (CallFunction|Move -1.0 -1.0 1.0 0.0)
                                  (goto _label Reset)
                                  (elif _returnvalue
                                    (CallFunction|Move -1.0 1.0 1.0 0.0)
                                    (goto _label Reset)
                                    (elif _returnvalue_3
                                      (CallFunction|Move 1.0 -1.0 1.0 0.0)
                                      (goto _label Reset)
                                      (elif _returnvalue_4
                                        (CallFunction|Move 1.0 1.0 1.0 0.0)
                                        (goto _label Reset)
                                        (else
                                          (goto _label Reset))))))))))))))))))))))

(event Input|EnhancedActionEvents|EnhancedInputActionAction
  (params (ActionValue :type Boolean) (ElapsedSeconds :type Float%20%28double-precision%29) (TriggeredSeconds :type Float%20%28double-precision%29) (InputAction :type Input%20Action%20Object%20Reference :default "/Game/PopFight/Blueprints/Player/input/Action.Action")))

(event Input|EnhancedActionEvents|EnhancedInputActionPause
  (params (ActionValue :type Boolean) (ElapsedSeconds :type Float%20%28double-precision%29) (TriggeredSeconds :type Float%20%28double-precision%29) (InputAction :type Input%20Action%20Object%20Reference :default "/Game/PopFight/Blueprints/Player/input/Pause.Pause")))

(event EventBeginPlay
  (Utilities|FlowControl|Sequence
    (:then_0
      (bind _asplayer_controller (Utilities|Casting|CastToPlayerController (Pawn|GetController)))
      (Utilities|IsValid (PlayerController|LocalPlayerSubsystems|GetEnhancedInputLocalPlayerSubsystem _asplayer_controller)
        (:Is%20Valid
          (Input|AddMappingContext (PlayerController|LocalPlayerSubsystems|GetEnhancedInputLocalPlayerSubsystem _asplayer_controller) "/Game/PopFight/Blueprints/Player/input/Balloon_Game_Input_Maping.Balloon_Game_Input_Maping" 0 "(bIgnoreAllPressedKeysUntilRelease=True,bForceImmediately=False,bNotifyUserSettings=False)"))))
    (:then_1
      (Utilities|Time|SetTimerbyEvent (delegate Custom|Ground%20Check) 0.2 true))))

(event Collision|EventActorBeginOverlap
  (params (OtherActor :type Actor%20Object%20Reference)))

(event EventTick
  (params (DeltaSeconds :type Float%20%28single-precision%29))
  (bind _sk_balloonanimal_01 (Variables|Default|Getsk_BalloonAnimal_01))
  (bind _returnvalue (Transformation|GetWorldLocation _sk_balloonanimal_01))
  (bind _returnvalue_2 (Collision|LineTraceByChannel _returnvalue (+ _returnvalue "0.000000,0.000000,-100.000000") "TraceTypeQuery1" false 0 "Persistent"))
  (if _returnvalue_2
    (Variables|Default|SetCan%20jump true)
    (else
      (Variables|Default|SetCan%20jump false))))

(event Input|KeyboardEvents|K
  (params (Key :type Key%20Structure :default "None"))
  (:Pressed
    (bind _outactors (Actor|GetAllActorswithInterface "/Game/PopFight/Clowns/ClownBlueprint/ClownInterface.ClownInterface_C"))
    (Class|ClownInterface|MakeMeLaugh(Message) _outactors)))

(fn ConstructionScript)

(fn Move
  (params (Left :type Float%20%28double-precision%29) (Forword :type Float%20%28double-precision%29) (Jump :type Float%20%28double-precision%29) (Clockwise :type Float%20%28double-precision%29))
  (bind _capsulecomponent (Variables|Collision|GetCapsuleComponent))
  (Physics|AddImpulse _capsulecomponent (Math|Vector|MakeVector 0.0 0.0 (* Jump (Variables|Default|GetJump_Hight))) "None" false)
  (Physics|AddImpulse _capsulecomponent (* (Transformation|GetActorRightVector) (* Left (Variables|Default|GetRight_Speed))) "None" false)
  (Physics|AddImpulse _capsulecomponent (* (Transformation|GetActorForwardVector) (* Forword (Variables|Default|GetForword_Speed))) "None" false)
  (Pawn|SetControlRotation (Pawn|GetController) (Math|Rotator|CombineRotators (Math|Rotator|MakeRotator 0.0 0.0 (* Clockwise (Variables|Default|GetYaw_Rate))) (Transformation|GetWorldRotation (Variables|Collision|GetCapsuleComponent)))))

(fn Hop
  (params (Jump%20Hight :type Float%20%28double-precision%29)))