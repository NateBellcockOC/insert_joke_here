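; Spawn point actor that places a respawnable balloon at its own location in PopFight.
; On BeginPlay it spawns a BP_Balloon at the root transform, passing it the spawner's point value, a respawnable flag and a reference back to itself.
; Its Respawn event waits a fixed delay, then spawns and configures a replacement balloon the same way.
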(event EventBeginPlay
  (bind _returnvalue (Game|SpawnActorfromClass "/Game/PopFight/Blueprints/BP_Balloon.BP_Balloon_C" (Transformation|GetWorldTransform (Variables|Default|GetDefaultSceneRoot)) "Undefined" "MultiplyWithRoot" 0 0))
  (Variables|/Game/PopFight/Blueprints/BP_Balloon.BP_Balloon_C|SetpointsWorth _returnvalue (Variables|Default|GetpointsWorth))
  (Variables|/Game/PopFight/Blueprints/BP_Balloon.BP_Balloon_C|SetIsRespawnable _returnvalue true)
  (Variables|/Game/PopFight/Blueprints/BP_Balloon.BP_Balloon_C|Setspawn _returnvalue self))

(event Collision|EventActorBeginOverlap
  (params (OtherActor :type Actor%20Object%20Reference)))

(event EventTick
  (params (DeltaSeconds :type Float%20%28single-precision%29)))

(event EventRespawn
  (Utilities|FlowControl|Delay 2e+01)
  (bind _returnvalue (Game|SpawnActorfromClass "/Game/PopFight/Blueprints/BP_Balloon.BP_Balloon_C" (Transformation|GetWorldTransform (Variables|Default|GetDefaultSceneRoot)) "Undefined" "MultiplyWithRoot" 0 0))
  (Variables|/Game/PopFight/Blueprints/BP_Balloon.BP_Balloon_C|SetpointsWorth _returnvalue (Variables|Default|GetpointsWorth))
  (Variables|/Game/PopFight/Blueprints/BP_Balloon.BP_Balloon_C|SetIsRespawnable _returnvalue true)
  (Variables|/Game/PopFight/Blueprints/BP_Balloon.BP_Balloon_C|Setspawn _returnvalue self))

(fn ConstructionScript)