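; BP_Balloon_Spawn_Temp is a one-shot spawn-point actor that places a BP_Balloon at its own transform after a random delay of a few seconds.
; It hands its SpawnNew reference to the new balloon, and calls Respawn on that reference if the balloon's Exists check is false.
; The actor then destroys itself, with all logic running from BeginPlay.
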(event EventBeginPlay
  (Utilities|FlowControl|Delay (Math|Random|RandomFloatinRange 0.0 5.0))
  (bind _returnvalue (Game|SpawnActorfromClass "/Game/PopFight/Blueprints/BP_Balloon.BP_Balloon_C" (Transformation|GetWorldTransform (Variables|Default|GetDefaultSceneRoot)) "Undefined" "MultiplyWithRoot" 0 0))
  (Variables|/Game/PopFight/Blueprints/BP_Balloon.BP_Balloon_C|SetspawnNew _returnvalue (Variables|Default|GetspawnNew))
  (if (Variables|/Game/PopFight/Blueprints/BP_Balloon.BP_Balloon_C|Getexists _returnvalue)
    _
    (else
      (Default|Respawn (Variables|Default|GetspawnNew))))
  (Actor|DestroyActor))

(event Collision|EventActorBeginOverlap
  (params (OtherActor :type Actor%20Object%20Reference)))

(event EventTick
  (params (DeltaSeconds :type Float%20%28single-precision%29)))

(fn ConstructionScript)