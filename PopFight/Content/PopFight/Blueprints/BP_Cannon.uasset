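; BP_Cannon is a cannon actor that fires characters out when they touch it.
; On Box overlap, any Character is moved to the box's location and rotation.
; Only a BP_ThirdPersonCharacter is then launched along the Arrow's forward vector at a fixed speed, overriding existing velocity, with a cannon sound played at the box.
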(event OnComponentBeginOverlap(Box)
  (params (OverlappedComponent :type Primitive%20Component%20Object%20Reference) (OtherActor :type Actor%20Object%20Reference) (OtherComp :type Primitive%20Component%20Object%20Reference) (OtherBodyIndex :type Integer) (bFromSweep :type Boolean) (SweepResult :type Hit%20Result%20Structure%20%28by%20ref%29))
  (bind _box (Variables|Default|GetBox))
  (bind _ascharacter (Utilities|Casting|CastToCharacter OtherActor))
  (Transformation|SetActorLocationAndRotation _ascharacter (Transformation|GetWorldLocation _box) (Transformation|GetWorldRotation _box))
  (Utilities|Casting|CastToBP_ThirdPersonCharacter _ascharacter)
  (Character|LaunchCharacter _ascharacter (* (Math|Vector|GetForwardVector (Variables|Default|GetArrow)) (Math|Conversions|ToVector(Float) 2000)) true true)
  (Audio|PlaySoundatLocation "/Game/PopFight/Audio/SoundFX/Canon.Canon" (Transformation|GetWorldLocation (Variables|Default|GetBox)) "0, 0, 0" 1.0 1.0 0.0 0 0 0 0))

(event EventBeginPlay)

(event Collision|EventActorBeginOverlap
  (params (OtherActor :type Actor%20Object%20Reference)))

(fn ConstructionScript)